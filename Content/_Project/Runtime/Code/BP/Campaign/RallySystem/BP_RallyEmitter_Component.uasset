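; Rally emitter component for the campaign rally system that provides visual and audio feedback when a rally signal is emitted.
; JuicyEmitSignal spawns a Niagara effect and plays a sound at the world location and rotation of RallyEmitPoint.
; Each effect runs only when the emit point and its own asset are valid, so a missing effect or sound does not block the other.
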(event `self.JuicyEmitSignal`
  (bind _rallyemitpoint (`self.RallyEmitPoint`))
  (bind _rallyemitpoint_2 (`self.RallyEmitPoint`))
  (`|ExecutionSequence`
    (:`then_0`
      (if (and (`KismetSystemLibrary.IsValid` (`self.RallyEmitPoint`)) (`KismetSystemLibrary.IsValid` (`self.NiagaraSystemTemplate`)))
        (`NiagaraFunctionLibrary.SpawnSystemAtLocation` (`self.NiagaraSystemTemplate`) (`SceneComponent.K2_GetComponentLocation` _rallyemitpoint) (`SceneComponent.K2_GetComponentRotation` _rallyemitpoint))))
    (:`then_1`
      (if (and (`KismetSystemLibrary.IsValid` (`self.RallyEmitPoint`)) (`KismetSystemLibrary.IsValid` (`self.RallyEmitSound`)))
        (`GameplayStatics.PlaySoundAtLocation` (`self.RallyEmitSound`) (`SceneComponent.K2_GetComponentLocation` _rallyemitpoint_2) (`SceneComponent.K2_GetComponentRotation` _rallyemitpoint_2) 1.0 1.0 0.0 null null null null)))))