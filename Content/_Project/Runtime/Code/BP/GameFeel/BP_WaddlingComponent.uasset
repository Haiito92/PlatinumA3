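; Game-feel component that produces a waddling motion by tweening the relative rotation of a target scene component.
; Starting it runs a custom-curve rotator tween with configurable delay, looping and yoyo, provided the duration is positive.
; Per-axis override flags choose whether roll, pitch and yaw follow the tween or keep their current value.
; Stopping pauses the stored tween task, and starting again resumes it.
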(event `self.ReceiveStartGamefeelComponent`
  (bind _modifiedscenecomponent (`self.ModifiedSceneComponent`))
  (bind (_relativerotation_roll _relativerotation_pitch _relativerotation_yaw) (`KismetMathLibrary.BreakRotator` (`SceneComponent.RelativeRotation` _modifiedscenecomponent)))
  (`/Engine/EditorBlueprintResources/StandardMacros.IsValid` (`self.WaddlingTask`)
    (:`Is Valid`
      (`FCTweenBPAction.Unpause` (`self.WaddlingTask`)))
    (:`Is Not Valid`
      (if (> (`self.Duration`) 0.0)
        (bind (_asynctaskproxy _value) (`FCTweenBPActionRotator.TweenRotatorCustomCurve` (`self.StartRotation`) (`self.EndRotation`) (`self.Duration`) (`self.AnimationCurve`) (`self.Delay`) (`KismetMathLibrary.SelectInt` -1 (`self.NbLoop`) (`self.Looping`)) (`self.Loop Delay`) (`self.Yoyoing`) (`self.Yoyo Delay`))
          (:`then`
            (set `self.WaddlingTask` _asynctaskproxy))
          (:`ApplyEasing`
            (`/Engine/EditorBlueprintResources/StandardMacros.IsValid` _modifiedscenecomponent
              (:`Is Valid`
                (`SceneComponent.K2_SetRelativeRotation` _modifiedscenecomponent (`KismetMathLibrary.MakeRotator` (`KismetMathLibrary.SelectFloat` (.roll _value) _relativerotation_roll (`self.OverrideX`)) (`KismetMathLibrary.SelectFloat` (.pitch _value) _relativerotation_pitch (`self.OverrideY`)) (`KismetMathLibrary.SelectFloat` (.yaw _value) _relativerotation_yaw (`self.OverrideZ`))) true false)))))))))

(event `self.ReceiveStopGamefeelComponent`
  (bind _waddlingtask (`self.WaddlingTask`))
  (`/Engine/EditorBlueprintResources/StandardMacros.IsValid` _waddlingtask
    (:`Is Valid`
      (`FCTweenBPAction.Pause` _waddlingtask))))