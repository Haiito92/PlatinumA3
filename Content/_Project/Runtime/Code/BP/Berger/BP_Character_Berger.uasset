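; BP_Character_Berger is the Berger character Blueprint, with placeholder reactions to being bitten and to the holding input.
; Its Bite event prints a hurt message and makes the character jump, using a boolean and a short delay to ignore repeat bites.
; The IA_Characters_Holding Enhanced Input action only prints a debug message when started.
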(event `self.ReceiveBeginPlay`)

(event `self.Bite`
  (if (not (`self.AlreadyBite`))
    (`KismetSystemLibrary.PrintString` "I'm Hurt " true true (struct :`R` 1.0 :`A` 1.0))
    (`self.Jump`)
    (set `self.AlreadyBite` true)
    (`KismetSystemLibrary.Delay` 1.0)
    (set `self.AlreadyBite` false)))

(event `EnhancedInput|/StateMachine/Characters/Common/NewInputs/IA_Characters_Holding`
  (params (ActionValue :type Boolean) (ElapsedSeconds :type "Float (double-precision)") (TriggeredSeconds :type "Float (double-precision)") (InputAction :type "InputAction Object Reference" :default "/StateMachine/Characters/Common/NewInputs/IA_Characters_Holding.IA_Characters_Holding"))
  (:`Started`
    (`KismetSystemLibrary.PrintString` "HOLDING")))

(fn `UserConstructionScript`
  (`parent.UserConstructionScript`))