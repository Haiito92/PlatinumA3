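; BP_Bush is a bush that releases a wolf once enough chase targets gather inside its sphere.
; Sphere overlaps maintain a SheepList of BP_WolfChasingTargetPlaceHolder actors, checked against a threshold on each entry.
; The first trigger spawns a hidden BP_Wolf facing the latest target, then reveals it after a delay, links it to the bush and starts the chase.
; Later triggers reuse that wolf when IsChasing is false.
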(event `self.Sphere.OnComponentBeginOverlap`
  (params (OverlappedComponent :type "PrimitiveComponent Object Reference") (OtherActor :type "Actor Object Reference") (OtherComp :type "PrimitiveComponent Object Reference") (OtherBodyIndex :type Integer) (bFromSweep :type Boolean) (SweepResult :type "HitResult Structure (by ref)"))
  (bind _sheeplist (`self.SheepList`))
  (bind _wolf (`self.Wolf`))
  (bind _asbp_wolf_chasing_target_place_holder (cast `/Game/_Project/Runtime/Code/BP/Wolf/BP_WolfChasingTargetPlaceHolder` OtherActor))
  (bind _output_get (set `self.As BP Wolf Chasing Target Place Holder` _asbp_wolf_chasing_target_place_holder))
  (`KismetArrayLibrary.Array_Add` _sheeplist _output_get)
  (if (>= (`KismetArrayLibrary.Array_Length` _sheeplist) (`self.NbMoutonsPourActiver`))
    (if (`self.hasSpawned`)
      (if (not (`self.isChasing`))
        (`self.SetActorHiddenInGame` _wolf false)
        (`/Game/_Project/Runtime/Code/BP/Wolf/BP_Wolf.CE_StartChasing` _wolf))
      (else
        (`self.SpawnWolf` (`self.WolfSpawnDelay`))
        (set `self.hasSpawned` true)))))

(event `SpawnWolf`
  (params (WolfSpawnDelay :type "Float (double-precision)"))
  (bind _returnvalue (`|SpawnActorFromClass` "/Game/_Project/Runtime/Code/BP/Wolf/BP_Wolf.BP_Wolf_C" (`KismetAnimationLibrary.K2_LookAt` (`self.GetTransform`) (`self.K2_GetActorLocation` (`self.As BP Wolf Chasing Target Place Holder`)) (`self.GetActorForwardVector`)) "Undefined" "MultiplyWithRoot" null null))
  (`self.SetActorHiddenInGame` _returnvalue true)
  (`KismetSystemLibrary.Delay` WolfSpawnDelay)
  (`self.SetActorHiddenInGame` _returnvalue false)
  (bind _output_get (set `self.Wolf` _returnvalue))
  (set `/Game/_Project/Runtime/Code/BP/Wolf/BP_Wolf.Bush` self _output_get)
  (`/Game/_Project/Runtime/Code/BP/Wolf/BP_Wolf.CE_StartChasing` (`self.Wolf`))
  (set `self.isChasing` true))

(event `self.Sphere.OnComponentEndOverlap`
  (params (OverlappedComponent :type "PrimitiveComponent Object Reference") (OtherActor :type "Actor Object Reference") (OtherComp :type "PrimitiveComponent Object Reference") (OtherBodyIndex :type Integer))
  (bind _asbp_wolf_chasing_target_place_holder (cast `/Game/_Project/Runtime/Code/BP/Wolf/BP_WolfChasingTargetPlaceHolder` OtherActor))
  (`KismetArrayLibrary.Array_RemoveItem` (`self.SheepList`) _asbp_wolf_chasing_target_place_holder))

(fn `Caught`
  (params (BushLocation :type "Vector Structure" :default (0.0 0.0 0.0))))

(fn `UserConstructionScript`)