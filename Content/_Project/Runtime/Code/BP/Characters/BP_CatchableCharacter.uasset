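; Character Blueprint that can be caught and launched, with its capsule component serving as the physics body.
; Catch prints a debug message and returns the capsule component to the caller.
; Launch sets the capsule's physics simulation and collision profile after a caller-supplied delay.
; In parallel, Launch runs a fast looping timer for a few seconds that interpolates capsule rotation back to zero.
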(event `self.Launch`
  (params (IsSimulatingPhysic :type Boolean) (CollisionProfilName :type Name) (TransTime :type "Float (single-precision)"))
  (`|ExecutionSequence`
    (:`then_0`
      (`KismetSystemLibrary.Delay` TransTime)
      (`PrimitiveComponent.SetSimulatePhysics` (`self.CapsuleComponent`) IsSimulatingPhysic)
      (`PrimitiveComponent.SetCollisionProfileName` (`self.CapsuleComponent`) CollisionProfilName true))
    (:`then_1`
      (bind _returnvalue (`KismetSystemLibrary.K2_SetTimer` null "LerpBackToNormal" 0.01 true))
      (set `self.LerpTimer` _returnvalue)
      (`KismetSystemLibrary.Delay` 4.0)
      (`KismetSystemLibrary.K2_ClearAndInvalidateTimerHandle` (`self.LerpTimer`)))))

(fn `Catch`
  (returns (ReturnValue :type "PrimitiveComponent Object Reference"))
  (`KismetSystemLibrary.PrintString` "SENDING PRIMITIVE")
  (return (`self.CapsuleComponent`)))

(fn `LerpBackToNormal`
  (`SceneComponent.K2_SetWorldRotation` (`self.CapsuleComponent`) (`KismetMathLibrary.RInterpTo` (`SceneComponent.K2_GetComponentRotation` (`self.CapsuleComponent`)) (struct) (`GameplayStatics.GetWorldDeltaSeconds`) 10.0) false false))

(fn `UserConstructionScript`)