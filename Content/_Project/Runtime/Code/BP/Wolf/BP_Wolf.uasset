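; BP_Wolf is an AI wolf character that chases, bites, then heads back.
; Chasing sets walk speed, flags the Blackboard and starts the jumpy-walk, waddling and squish-squash components for procedural movement feel.
; Bite halts movement and those effects, plays a sound and starts a timer.
; The timer's Stun event, despite its name, restores speed and effects and sets the isComingBack Blackboard key.
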(event `CE_StartChasing`
  (params (ChaseSpeed :type "Float (double-precision)"))
  (set `self.WolfMaxWalkSpeed` ChaseSpeed)
  (set `CharacterMovementComponent.MaxWalkSpeed` ChaseSpeed (`self.CharacterMovement`))
  (set `self.isChasing` true)
  (`BlackboardComponent.SetValueAsBool` (`AIBlueprintHelperLibrary.GetBlackboard` null) "isChasing" true)
  (`JumpyWalkComponent.StartJumpyWalk` (`self.BP_JumpyWalkComponent`))
  (`WaddlingComponent.StartWaddling` (`self.BP_WaddlingComponent`))
  (`SquishSquashComponent.StartSquishSquash` (`self.Bp_SquishSquashComponent`)))

(event `self.Bite`
  (params (StunTimer :type "Float (single-precision)"))
  (`KismetSystemLibrary.PrintString` "bite")
  (if (not (`self.Bitten`))
    (`JumpyWalkComponent.StopJumpyWalk` (`self.BP_JumpyWalkComponent`))
    (`WaddlingComponent.StopWaddling` (`self.BP_WaddlingComponent`))
    (`SquishSquashComponent.StopSquishSquash` (`self.Bp_SquishSquashComponent`))
    (set `self.Bitten` true)
    (set `CharacterMovementComponent.MaxWalkSpeed` 0.0 (`self.CharacterMovement`))
    (`KismetSystemLibrary.K2_SetTimerDelegate` (delegate `Stun`) 2.0)
    (`self.JUICY_Bitten`)))

(event `Stun`
  (`BlackboardComponent.SetValueAsBool` (`AIBlueprintHelperLibrary.GetBlackboard` null) "isComingBack" true)
  (set `self.Bitten` false)
  (set `CharacterMovementComponent.MaxWalkSpeed` (`self.WolfMaxWalkSpeed`) (`self.CharacterMovement`))
  (`JumpyWalkComponent.StartJumpyWalk` (`self.BP_JumpyWalkComponent`))
  (`WaddlingComponent.StartWaddling` (`self.BP_WaddlingComponent`))
  (`SquishSquashComponent.StartSquishSquash` (`self.Bp_SquishSquashComponent`)))

(event `JUICY_Bitten`
  ;[1 1 1] JUICY_Bitten
  (`GameplayStatics.SpawnSoundAtLocation` null (`self.K2_GetActorLocation`) (struct) 1.0 1.0 0.0 null null))

(fn `UserConstructionScript`)