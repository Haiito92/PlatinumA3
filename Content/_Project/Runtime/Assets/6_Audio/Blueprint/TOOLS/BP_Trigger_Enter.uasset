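; BP_Trigger_Enter is an audio trigger that plays a one-shot sound when the shepherd (Berger) or dog (Chien) character enters it.
; On actor overlap it casts to each character in turn, spawns the Sound variable at that character's location and prints a debug message.
; The DoOnce gate sits before the casts, so the first overlap by any actor uses up the trigger.
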(event `self.ReceiveActorBeginOverlap`
  (params (OtherActor :type "Actor Object Reference"))
  (`/Engine/EditorBlueprintResources/StandardMacros.DoOnce` false
    (:`Completed`
      (bind _asbp_character_berger (cast `/Game/_Project/Runtime/Code/BP/Characters/Berger/BP_Character_Berger` OtherActor)
        (:`then`
          (`GameplayStatics.SpawnSoundAtLocation` (`self.Sound`) (`self.K2_GetActorLocation` _asbp_character_berger) (struct) 1.0 1.0 0.0 null null)
          (`KismetSystemLibrary.PrintString` "Audio Enter Shepherd" true true (struct :`R` 1.0 :`G` 1.0 :`B` 1.0 :`A` 1.0)))
        (:`CastFailed`
          (bind _asbp_character_chien (cast `/Game/_Project/Runtime/Code/BP/Characters/Chien/BP_Character_Chien` OtherActor))
          (`GameplayStatics.SpawnSoundAtLocation` (`self.Sound`) (`self.K2_GetActorLocation` _asbp_character_chien) (struct) 1.0 1.0 0.0 null null)
          (`KismetSystemLibrary.PrintString` "Audio Enter Dog" true true (struct :`R` 1.0 :`G` 1.0 :`B` 1.0 :`A` 1.0)))))))

(fn `UserConstructionScript`)