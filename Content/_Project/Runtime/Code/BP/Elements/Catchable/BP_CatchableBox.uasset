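; BP_CatchableBox is a catchable box element whose Cube component is handed to whatever catches it.
; Catch fires the JUICYOnCatched event and returns the Cube, while Cube hits fire JUICYOnCollided; both events are empty hooks for feedback.
; Every Tick, its Widget component is rotated to face the first player's camera, billboard style.
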(event `Event JUICY On Catched`)

(event `Event JUICY On Collided`)

(event `self.Cube.OnComponentHit`
  (params (HitComponent :type "PrimitiveComponent Object Reference") (OtherActor :type "Actor Object Reference") (OtherComp :type "PrimitiveComponent Object Reference") (NormalImpulse :type "Vector Structure") (Hit :type "HitResult Structure (by ref)"))
  (`self.Event JUICY On Collided`))

(event `self.ReceiveTick`
  (params (DeltaSeconds :type "Float (single-precision)"))
  (bind _returnvalue (`GameplayStatics.GetPlayerController` 0))
  (bind _playercameramanager (`PlayerController.PlayerCameraManager` _returnvalue))
  (`/Engine/EditorBlueprintResources/StandardMacros.IsValid` _returnvalue
    (:`Is Valid`
      (`/Engine/EditorBlueprintResources/StandardMacros.IsValid` _playercameramanager
        (:`Is Valid`
          (`SceneComponent.K2_SetWorldRotation` (`self.Widget`) (`KismetMathLibrary.Conv_VectorToRotator` (- (`PlayerCameraManager.GetCameraLocation` _playercameramanager) (`SceneComponent.K2_GetComponentLocation` (`self.Widget`)))) false false))))))

(fn `Catch`
  (returns (ReturnValue :type "PrimitiveComponent Object Reference"))
  (`self.Event JUICY On Catched`)
  (return (`self.Cube`)))

(fn `UserConstructionScript`)