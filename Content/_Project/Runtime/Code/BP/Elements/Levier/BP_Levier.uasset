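; BP_Levier is a lever element that relays an interaction to a linked InteractedObject.
; Interact calls InteractMessage on that object if it is valid and implements InteractInterface, and BeginPlay fires it once when ISON is set.
; Tick rotates the Widget component to face the player camera.
; The construction script applies the exposed radius and intensity settings to the PointLight.
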(event `self.ReceiveBeginPlay`
  (if (`self.IS_ON`)
    (`self.Interact` null)))

(event `InteractInterface.Interact`
  (params (PlayerInteracting :type "PlayerController Object Reference"))
  (bind _interactedobject (`self.InteractedObject`))
  (`/Engine/EditorBlueprintResources/StandardMacros.IsValid` _interactedobject
    (:`Is Valid`
      (if (`KismetSystemLibrary.DoesImplementInterface` _interactedobject "/Script/PlatinumA3.InteractInterface")
        (message `InteractInterface.Interact` (`self.InteractedObject`) null)))))

(event `self.ReceiveTick`
  (params (DeltaSeconds :type "Float (single-precision)"))
  (bind _returnvalue (`GameplayStatics.GetPlayerController` 0))
  (bind _playercameramanager (`PlayerController.PlayerCameraManager` _returnvalue))
  (`/Engine/EditorBlueprintResources/StandardMacros.IsValid` _returnvalue
    (:`Is Valid`
      (`/Engine/EditorBlueprintResources/StandardMacros.IsValid` _playercameramanager
        (:`Is Valid`
          (`SceneComponent.K2_SetWorldRotation` (`self.Widget`) (`KismetMathLibrary.Conv_VectorToRotator` (- (`PlayerCameraManager.GetCameraLocation` _playercameramanager) (`SceneComponent.K2_GetComponentLocation` (`self.Widget`)))) false false))))))

(fn `UserConstructionScript`
  (`LocalLightComponent.SetAttenuationRadius` (`self.PointLight`) (`self.LIGHT_AttenuationRadius`))
  (`PointLightComponent.SetSourceRadius` (`self.PointLight`) (`self.LIGHT_SourceRadius`))
  (`LightComponent.SetIntensity` (`self.PointLight`) (`self.LIGHT_Intensity`)))