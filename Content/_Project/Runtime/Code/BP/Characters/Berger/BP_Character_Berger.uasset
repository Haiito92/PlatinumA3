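; Shepherd (Berger) character Blueprint that maps Enhanced Input to holding and launching, rallying with an emitted signal, and interacting.
; Jumpy-walk, squish-squash and waddling gamefeel components are initialized on the mesh, then started and stopped by character movement delegates.
; Landing spawns a fall Niagara effect, and JUICY hooks play sounds for holding and throwing.
; Bite triggers a hurt debug print and a jump, gated by a one-second cooldown.
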(event `self.ReceiveBeginPlay`
  (add `self.LandedDelegate` (delegate `LandedDelegate_Event`))
  (add `StateCharacter.CharacterStartMove_Delegate` (`|CreateDelegate` :!event `OnCharacterStartMove`))
  (add `StateCharacter.CharacterStopMove_Delegate` (`|CreateDelegate` :!event `OnCharacterStopMove`))
  (`|ExecutionSequence`
    (:`then_0`
      (`GamefeelComponent.InitGamefeelComponent` (`self.BP_JumpyWalkComponent`) (`self.Mesh`))
      (set `/Game/_Project/Runtime/Code/BP/GameFeel/BP_JumpyWalkComponent.FootstepPoint` (`self.FootstepPoint`) (`self.BP_JumpyWalkComponent`)))
    (:`then_1`
      (`GamefeelComponent.InitGamefeelComponent` (`self.Bp_SquishSquashComponent`) (`self.Mesh`)))
    (:`then_2`
      (`GamefeelComponent.InitGamefeelComponent` (`self.BP_WaddlingComponent`) (`self.Mesh`)))))

(event `LandedDelegate_Event` :!signature `self.LandedDelegate`
  (params (Hit :type "HitResult Structure (by ref)"))
  (`NiagaraFunctionLibrary.SpawnSystemAtLocation` "/Game/VFX/VFX_Walk/NS_Fall.NS_Fall" (`.ImpactPoint` (`GameplayStatics.BreakHitResult` Hit))))

(event `self.Bite`
  (params (StunTimer :type "Float (single-precision)"))
  (if (not (`self.AlreadyBite`))
    (`KismetSystemLibrary.PrintString` "I'm Hurt " true true (struct :`R` 1.0 :`A` 1.0))
    (`self.Jump`)
    (set `self.AlreadyBite` true)
    (`KismetSystemLibrary.Delay` 1.0)
    (set `self.AlreadyBite` false)))

(event `EnhancedInput|/StateMachine/Characters/Common/NewInputs/IA_Characters_Holding`
  (params (ActionValue :type Boolean) (ElapsedSeconds :type "Float (double-precision)") (TriggeredSeconds :type "Float (double-precision)") (InputAction :type "InputAction Object Reference" :default "/StateMachine/Characters/Common/NewInputs/IA_Characters_Holding.IA_Characters_Holding"))
  (:`Started`
    (`self.StartHolding`))
  (:`Completed`
    (`self.LaunchSomething`)))

(event `EnhancedInput|/StateMachine/Characters/Common/NewInputs/IA_Characters_Launching`
  (params (ActionValue :type Boolean) (ElapsedSeconds :type "Float (double-precision)") (TriggeredSeconds :type "Float (double-precision)") (InputAction :type "InputAction Object Reference" :default "/StateMachine/Characters/Common/NewInputs/IA_Characters_Launching.IA_Characters_Launching")))

(event `EnhancedInput|/StateMachine/Characters/Common/NewInputs/IA_Characters_Rallying`
  (params (ActionValue :type Boolean) (ElapsedSeconds :type "Float (double-precision)") (TriggeredSeconds :type "Float (double-precision)") (InputAction :type "InputAction Object Reference" :default "/StateMachine/Characters/Common/NewInputs/IA_Characters_Rallying.IA_Characters_Rallying"))
  (:`Started`
    (`KismetSystemLibrary.PrintString` "Launch Rally")
    (`self.LaunchRally`)
    (`RallyEmitterComponent.EmitSignal` (`self.RallyEmitter`))))

(event `EnhancedInput|/StateMachine/Characters/Common/NewInputs/IA_Characters_Interacting`
  (params (ActionValue :type Boolean) (ElapsedSeconds :type "Float (double-precision)") (TriggeredSeconds :type "Float (double-precision)") (InputAction :type "InputAction Object Reference" :default "/StateMachine/Characters/Common/NewInputs/IA_Characters_Interacting.IA_Characters_Interacting"))
  (:`Started`
    (`self.LaunchInteracting`)
    (`KismetSystemLibrary.PrintString` "Interacting")))

(event `self.JUICY_OnInteract`)

(event `self.JUICY_OnThrowSomething`
  (`GameplayStatics.PlaySoundAtLocation` null (`self.K2_GetActorLocation`) (struct) 1.0 1.0 0.0 null null null null))

(event `self.JUICY_OnStartHolding`
  (`GameplayStatics.PlaySoundAtLocation` null (`self.K2_GetActorLocation`) (struct) 1.0 1.0 0.0 null null null null))

(event `OnCharacterStartMove`
  (`GamefeelComponent.StartGamefeelComponent` (`self.BP_JumpyWalkComponent`))
  (`GamefeelComponent.StartGamefeelComponent` (`self.Bp_SquishSquashComponent`))
  (`GamefeelComponent.StartGamefeelComponent` (`self.BP_WaddlingComponent`)))

(event `OnCharacterStopMove`
  (`GamefeelComponent.StopGamefeelComponent` (`self.BP_JumpyWalkComponent`))
  (`GamefeelComponent.StopGamefeelComponent` (`self.Bp_SquishSquashComponent`))
  (`GamefeelComponent.StopGamefeelComponent` (`self.BP_WaddlingComponent`)))

(fn `UserConstructionScript`
  (`parent.UserConstructionScript`))