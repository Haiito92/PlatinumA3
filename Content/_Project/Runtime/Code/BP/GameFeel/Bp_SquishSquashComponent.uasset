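; Game-feel component that animates a target object's world scale between squish and squash values.
; Start creates a curve-driven vector tween with configurable delay, looping (optionally infinite) and yoyo, or unpauses the stored task if it is still valid.
; Stop only pauses that task.
; Each loop fires JuicySquishSquash, an event with an empty body here.
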(event `self.StartSquishSquash`
  (bind _squishsquashedobject (`self.SquishSquashedObject`))
  (`/Engine/EditorBlueprintResources/StandardMacros.IsValid` (`self.SquishSquashTask`)
    (:`Is Valid`
      (`FCTweenBPAction.Unpause` (`self.SquishSquashTask`)))
    (:`Is Not Valid`
      (bind (_asynctaskproxy _value) (`FCTweenBPActionVector.TweenVectorCustomCurve` (`self.StartSquish`) (`self.EndSquash`) (`self.Duration`) (`self.AnimationCurve`) (`self.Delay`) (`KismetMathLibrary.SelectInt` -1 (`self.NbLoop`) (`self.Looping`)) (`self.Loop Delay`) (`self.Yoyoing`) (`self.Yoyo Delay`))
        (:`then`
          (set `self.SquishSquashTask` _asynctaskproxy))
        (:`ApplyEasing`
          (`/Engine/EditorBlueprintResources/StandardMacros.IsValid` _squishsquashedobject
            (:`Is Valid`
              (`SceneComponent.SetWorldScale3D` _squishsquashedobject _value))))
        (:`OnLoop`
          (`self.JuicySquishSquash`))))))

(event `self.StopSquishSquash`
  (`FCTweenBPAction.Pause` (`self.SquishSquashTask`)))

(event `self.JuicySquishSquash`)