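; Main menu HUD that sets up the menu and character selection screens for up to two local players.
; On BeginPlay it creates the main menu widget and the character selection widget and adds both to the viewport, with selection starting collapsed.
; The selection's P0 sub-widget is owned by player controller 0, and P1 by controller 1 only if that controller exists.
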(event `self.ReceiveBeginPlay`
  (bind _returnvalue (`GameplayStatics.GetPlayerController` 1))
  (bind _selectionpersonnage (`self.SelectionPersonnage`))
  (bind _returnvalue_2 (`|CreateWidget` "/Game/_Project/Runtime/Code/Widget/W_MainMenu.W_MainMenu_C"))
  (bind _output_get (set `self.MainMenu` _returnvalue_2))
  (`UserWidget.AddToViewport` _output_get 0)
  (bind _returnvalue_3 (`|CreateWidget` "/Game/_Project/Runtime/Code/Widget/W_PersoSelection.W_PersoSelection_C" (`GameplayStatics.GetPlayerController` 0)))
  (bind _output_get_2 (set `self.SelectionPersonnage` _returnvalue_3))
  (`Widget.SetVisibility` _output_get_2 "Collapsed")
  (`UserWidget.AddToViewport` _output_get_2 0)
  (`UserWidget.SetOwningPlayer` (`/Game/_Project/Runtime/Code/Widget/W_PersoSelection.P0` _selectionpersonnage) (`GameplayStatics.GetPlayerController` 0))
  (if (`KismetSystemLibrary.IsValid` _returnvalue)
    (`UserWidget.SetOwningPlayer` (`/Game/_Project/Runtime/Code/Widget/W_PersoSelection.P1` _selectionpersonnage) _returnvalue)))

(fn `UserConstructionScript`)