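; Drawbridge ("pont-levis") actor that rotates into a target orientation when activated.
; Interact runs a three-second rotator tween from the Transform component's world rotation to that of TargetTransform, applying each eased value as world rotation.
; If the ISON flag is set, BeginPlay triggers Interact automatically; the rotation only goes toward the target, with no return path.
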(event `self.ReceiveBeginPlay`
  (if (`self.IS_ON`)
    (`self.Interact` null)))

(event `InteractInterface.Interact`
  (params (PlayerInteracting :type "PlayerController Object Reference"))
  (bind (_asynctaskproxy _value) (`FCTweenBPActionRotator.TweenRotator` (`SceneComponent.K2_GetComponentRotation` (`self.Transform`)) (`SceneComponent.K2_GetComponentRotation` (`self.TargetTransform`)) 3.0)
    (:`ApplyEasing`
      (`SceneComponent.K2_SetWorldRotation` (`self.Transform`) _value false false))))

(fn `UserConstructionScript`)