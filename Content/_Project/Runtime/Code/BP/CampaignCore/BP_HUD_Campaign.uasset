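; Campaign HUD Blueprint that spawns the UI widgets for a campaign session.
; One tick after BeginPlay, and only for player controller ID 0, it adds the campaign overlay, a start menu with keyboard focus, a collapsed global pause menu and a hidden cheats menu.
; A GameFinished event creates, initializes and shows the end menu for the owning player.
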(event `self.ReceiveBeginPlay`
  (`KismetSystemLibrary.DelayUntilNextTick`)
  (if (== (`GameplayStatics.GetPlayerControllerID` (`self.PlayerOwner`)) 0)
    (`|ExecutionSequence`
      (:`then_0`
        (bind _returnvalue (`|CreateWidget` "/Game/_Project/Runtime/Code/Widget/Campaign/WBP_CampaignOverlay.WBP_CampaignOverlay_C" (`self.PlayerOwner`)))
        (`UserWidget.AddToViewport` _returnvalue 0)
        (`CampaignOverlay.InitCampaignOverlay` _returnvalue)
        (bind _returnvalue_2 (`|CreateWidget` "/Game/_Project/Runtime/Code/Widget/W_StartMenu.W_StartMenu_C"))
        (`UserWidget.AddToViewport` _returnvalue_2 0)
        (`Widget.SetKeyboardFocus` (`/Game/_Project/Runtime/Code/Widget/W_StartMenu.Understoodbutton` _returnvalue_2))
        (bind _returnvalue_3 (`|CreateWidget` "/Game/_Project/Runtime/Code/Widget/PauseMenuGlobal.PauseMenuGlobal_C"))
        (`UserWidget.AddToViewport` _returnvalue_3 0)
        (`Widget.SetVisibility` _returnvalue_3 "Collapsed"))
      (:`then_1`
        (bind _returnvalue_4 (`|CreateWidget` "/Game/_Project/Runtime/Code/Widget/CheatsSystem/WBP_CheatsMenu.WBP_CheatsMenu_C" (`self.PlayerOwner`)))
        (`Widget.SetVisibility` _returnvalue_4 "Hidden")
        (`UserWidget.AddToViewport` _returnvalue_4 0)
        (`CheatsMenu.InitCheatsMenu` _returnvalue_4)))))

(event `self.ReceiveGameFinished`
  (`KismetSystemLibrary.PrintString` "HUD END GAME" true true (struct :`G` 0.316667 :`B` 0.195274 :`A` 1.0) 4.0)
  (bind _returnvalue (`|CreateWidget` "/Game/_Project/Runtime/Code/Widget/W_EndMenu.W_EndMenu_C" (`self.PlayerOwner`)))
  (`EndGameMenu.InitEndGameMenu` _returnvalue)
  (`UserWidget.AddToViewport` _returnvalue 0))

(fn `UserConstructionScript`)