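; Trigger actor that starts the Play_Mus_IG music as a 2D sound when the Berger or Chien character enters one of its zones.
; Two boxes, EnterBox_01 and EnterBox_02, run identical overlap logic, casting the overlapping actor to either character class.
; A shared MusIsPlaying flag, cleared only at BeginPlay, limits the music to one start per actor lifetime, with no stop logic.
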(event `self.ReceiveBeginPlay`
  (set `self.MusIsPlaying` false))

(event `self.EnterBox_02.OnComponentBeginOverlap`
  (params (OverlappedComponent :type "PrimitiveComponent Object Reference") (OtherActor :type "Actor Object Reference") (OtherComp :type "PrimitiveComponent Object Reference") (OtherBodyIndex :type Integer) (bFromSweep :type Boolean) (SweepResult :type "HitResult Structure (by ref)"))
  (if (not (`self.MusIsPlaying`))
    (cast `/Game/_Project/Runtime/Code/BP/Characters/Berger/BP_Character_Berger` OtherActor
      (:`then`
        (`GameplayStatics.PlaySound2D` "/Game/_Project/Runtime/Assets/6_Audio/Event/Mus/Play_Mus_IG.Play_Mus_IG" 1.0 1.0 0.0 null null))
      (:`CastFailed`
        (cast `/Game/_Project/Runtime/Code/BP/Characters/Chien/BP_Character_Chien` OtherActor)
        (`GameplayStatics.PlaySound2D` "/Game/_Project/Runtime/Assets/6_Audio/Event/Mus/Play_Mus_IG.Play_Mus_IG" 1.0 1.0 0.0 null null)))
    (set `self.MusIsPlaying` true)))

(event `self.EnterBox_01.OnComponentBeginOverlap`
  (params (OverlappedComponent :type "PrimitiveComponent Object Reference") (OtherActor :type "Actor Object Reference") (OtherComp :type "PrimitiveComponent Object Reference") (OtherBodyIndex :type Integer) (bFromSweep :type Boolean) (SweepResult :type "HitResult Structure (by ref)"))
  (if (not (`self.MusIsPlaying`))
    (cast `/Game/_Project/Runtime/Code/BP/Characters/Berger/BP_Character_Berger` OtherActor
      (:`then`
        (`GameplayStatics.PlaySound2D` "/Game/_Project/Runtime/Assets/6_Audio/Event/Mus/Play_Mus_IG.Play_Mus_IG" 1.0 1.0 0.0 null null))
      (:`CastFailed`
        (cast `/Game/_Project/Runtime/Code/BP/Characters/Chien/BP_Character_Chien` OtherActor)
        (`GameplayStatics.PlaySound2D` "/Game/_Project/Runtime/Assets/6_Audio/Event/Mus/Play_Mus_IG.Play_Mus_IG" 1.0 1.0 0.0 null null)))
    (set `self.MusIsPlaying` true)))

(fn `UserConstructionScript`)