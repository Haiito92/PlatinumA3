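; Audio actor for hole ambience that spawns Play_AMB_Hole at its location when shepherd or dog characters overlap it.
; BeginPlay also spawns a sound at the origin with no asset assigned.
; Shepherd entry is gated on no valid dog sound, while dog entry requires a valid shepherd sound.
; With that sound valid, other overlapping actors send "Stop" to it from begin overlap, as no end-overlap handler exists.
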(event `self.ReceiveBeginPlay`
  (`/Engine/EditorBlueprintResources/StandardMacros.IsValid` (`self.Play`)
    (:`Is Not Valid`
      (bind _returnvalue (`GameplayStatics.SpawnSoundAtLocation` null (0.0 0.0 0.0) (struct) 1.0 1.0 0.0 null null))
      (set `self.Play` _returnvalue))))

(event `self.ReceiveActorBeginOverlap`
  (params (OtherActor :type "Actor Object Reference"))
  (cast `/Game/_Project/Runtime/Code/BP/Characters/Berger/BP_Character_Berger` OtherActor
    (:`then`
      (`/Engine/EditorBlueprintResources/StandardMacros.IsValid` (`self.PlayOnDog`)
        (:`Is Not Valid`
          (bind _returnvalue (`GameplayStatics.SpawnSoundAtLocation` "/Game/_Project/Runtime/Assets/6_Audio/Event/AMB/Night/Play_AMB_Hole.Play_AMB_Hole" (`self.K2_GetActorLocation`) (struct) 1.0 1.0 0.0 null null))
          (set `self.PlayOnShep` _returnvalue)
          (`KismetSystemLibrary.PrintString` "Audio_Hole_EnterSphere" true true (struct :`R` 1.0 :`G` 1.0 :`B` 1.0 :`A` 1.0)))))
    (:`CastFailed`
      (`/Engine/EditorBlueprintResources/StandardMacros.IsValid` (`self.PlayOnShep`)
        (:`Is Valid`
          (cast `/Game/_Project/Runtime/Code/BP/Characters/Chien/BP_Character_Chien` OtherActor
            (:`then`
              (bind _returnvalue_2 (`GameplayStatics.SpawnSoundAtLocation` "/Game/_Project/Runtime/Assets/6_Audio/Event/AMB/Night/Play_AMB_Hole.Play_AMB_Hole" (`self.K2_GetActorLocation`) (struct) 1.0 1.0 0.0 null null))
              (set `self.PlayOnDog` _returnvalue_2)
              (`KismetSystemLibrary.PrintString` "Audio_Hole_EnterSphere" true true (struct :`R` 1.0 :`G` 1.0 :`B` 1.0 :`A` 1.0)))
            (:`CastFailed`
              (`AudioParameterControllerInterface.SetTriggerParameter` _returnvalue "Stop")
              (`KismetSystemLibrary.PrintString` "Audio_Hole_ExitSphere" true true (struct :`R` 1.0 :`G` 1.0 :`B` 1.0 :`A` 1.0)))))))))

(fn `UserConstructionScript`)