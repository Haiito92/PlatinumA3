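; Main menu player controller that handles Enhanced Input for menu navigation and a hold-to-charge button.
; It forwards selection movement through the OnMoveMenuSelection event.
; Holding click increments HoldButtonValue while ChargedButton is enabled and stops the decay timeline.
; Releasing click restarts that timeline, which lerps the hold value back toward zero.
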(event `EnhancedInput|/Game/_Project/Runtime/Inputs/IA_MoveMenuSelection`
  (params (ActionValue :type "Float (double-precision)") (ElapsedSeconds :type "Float (double-precision)") (TriggeredSeconds :type "Float (double-precision)") (InputAction :type "InputAction Object Reference" :default "/Game/_Project/Runtime/Inputs/IA_MoveMenuSelection.IA_MoveMenuSelection"))
  (:`Started`
    (`self.OnMoveMenuSelection` ActionValue)))

(event `EnhancedInput|/Game/_Project/Runtime/Inputs/IA_ClickButton`
  (params (ActionValue :type Boolean) (ElapsedSeconds :type "Float (double-precision)") (TriggeredSeconds :type "Float (double-precision)") (InputAction :type "InputAction Object Reference" :default "/Game/_Project/Runtime/Inputs/IA_ClickButton.IA_ClickButton"))
  (:`Triggered`
    (if (`Widget.GetIsEnabled` (`self.ChargedButton`))
      (set `self.HoldButtonValue` (+ (`self.HoldButtonValue`) 1.0))
      (bind (_direction _0) (`Timeline|Decrease progress bar` :!via `Stop` :!label _label)
        (:`Update`
          (set `self.HoldButtonValue` (`KismetMathLibrary.Lerp` (`self.HoldButtonValue`) 0.0 _0))))))
  (:`Completed`
    (goto _label :!via `PlayFromStart`)))

(fn `UserConstructionScript`)