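; Audio trigger volume that plays the Teleporter 1 ambience and shifts the sound mix as the Berger character enters or leaves.
; The enter box spawns the sound at the actor's location unless one is still valid, and pushes the Teleporter_In mix over music, day/night ambience and NPC classes.
; Four exit boxes, gated by an inside flag, fire the sound's Stop trigger parameter and push the Teleporter_Out mix.
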(event `self.ReceiveBeginPlay`)

(event `self.Box_Exit_03.OnComponentBeginOverlap`
  (params (OverlappedComponent :type "PrimitiveComponent Object Reference") (OtherActor :type "Actor Object Reference") (OtherComp :type "PrimitiveComponent Object Reference") (OtherBodyIndex :type Integer) (bFromSweep :type Boolean) (SweepResult :type "HitResult Structure (by ref)"))
  ;[1 1 1] EXIT
  (cast `/Game/_Project/Runtime/Code/BP/Characters/Berger/BP_Character_Berger` OtherActor)
  (if (`self.isBergerInside`)
    (set `self.isBergerInside` false)
    (`AudioParameterControllerInterface.SetTriggerParameter` (`self.PlayOnShep`) "Stop")
    (`KismetSystemLibrary.PrintString` "Audio_Hole_ExitSphere" true true (struct :`R` 1.0 :`G` 1.0 :`B` 1.0 :`A` 1.0))
    (`GameplayStatics.SetSoundMixClassOverride` "/Game/_Project/Runtime/Assets/6_Audio/Mix/SoundMix/SFX/SoundMix_Teleporter_Out.SoundMix_Teleporter_Out" "/Game/_Project/Runtime/Assets/6_Audio/Mix/SoundClass/MIX_Class/MUS_IG.MUS_IG")
    (`GameplayStatics.SetSoundMixClassOverride` "/Game/_Project/Runtime/Assets/6_Audio/Mix/SoundMix/SFX/SoundMix_Teleporter_Out.SoundMix_Teleporter_Out" "/Game/_Project/Runtime/Assets/6_Audio/Mix/SoundClass/MIX_Class/AMB_Day_Mix.AMB_Day_Mix")
    (`GameplayStatics.SetSoundMixClassOverride` "/Game/_Project/Runtime/Assets/6_Audio/Mix/SoundMix/SFX/SoundMix_Teleporter_Out.SoundMix_Teleporter_Out" "/Game/_Project/Runtime/Assets/6_Audio/Mix/SoundClass/AMB_Night.AMB_Night")
    (`GameplayStatics.SetSoundMixClassOverride` "/Game/_Project/Runtime/Assets/6_Audio/Mix/SoundMix/SFX/SoundMix_Teleporter_Out.SoundMix_Teleporter_Out" "/Game/_Project/Runtime/Assets/6_Audio/Mix/SoundClass/MIX_Class/NPC_MIX.NPC_MIX")
    (`GameplayStatics.PushSoundMixModifier` "/Game/_Project/Runtime/Assets/6_Audio/Mix/SoundMix/SFX/SoundMix_Teleporter_Out.SoundMix_Teleporter_Out")))

(event `self.Box_Exit_04.OnComponentBeginOverlap`
  (params (OverlappedComponent :type "PrimitiveComponent Object Reference") (OtherActor :type "Actor Object Reference") (OtherComp :type "PrimitiveComponent Object Reference") (OtherBodyIndex :type Integer) (bFromSweep :type Boolean) (SweepResult :type "HitResult Structure (by ref)"))
  ;[1 1 1] EXIT
  (cast `/Game/_Project/Runtime/Code/BP/Characters/Berger/BP_Character_Berger` OtherActor)
  (if (`self.isBergerInside`)
    (set `self.isBergerInside` false)
    (`AudioParameterControllerInterface.SetTriggerParameter` (`self.PlayOnShep`) "Stop")
    (`KismetSystemLibrary.PrintString` "Audio_Hole_ExitSphere" true true (struct :`R` 1.0 :`G` 1.0 :`B` 1.0 :`A` 1.0))
    (`GameplayStatics.SetSoundMixClassOverride` "/Game/_Project/Runtime/Assets/6_Audio/Mix/SoundMix/SFX/SoundMix_Teleporter_Out.SoundMix_Teleporter_Out" "/Game/_Project/Runtime/Assets/6_Audio/Mix/SoundClass/MIX_Class/MUS_IG.MUS_IG")
    (`GameplayStatics.SetSoundMixClassOverride` "/Game/_Project/Runtime/Assets/6_Audio/Mix/SoundMix/SFX/SoundMix_Teleporter_Out.SoundMix_Teleporter_Out" "/Game/_Project/Runtime/Assets/6_Audio/Mix/SoundClass/MIX_Class/AMB_Day_Mix.AMB_Day_Mix")
    (`GameplayStatics.SetSoundMixClassOverride` "/Game/_Project/Runtime/Assets/6_Audio/Mix/SoundMix/SFX/SoundMix_Teleporter_Out.SoundMix_Teleporter_Out" "/Game/_Project/Runtime/Assets/6_Audio/Mix/SoundClass/AMB_Night.AMB_Night")
    (`GameplayStatics.SetSoundMixClassOverride` "/Game/_Project/Runtime/Assets/6_Audio/Mix/SoundMix/SFX/SoundMix_Teleporter_Out.SoundMix_Teleporter_Out" "/Game/_Project/Runtime/Assets/6_Audio/Mix/SoundClass/MIX_Class/NPC_MIX.NPC_MIX")
    (`GameplayStatics.PushSoundMixModifier` "/Game/_Project/Runtime/Assets/6_Audio/Mix/SoundMix/SFX/SoundMix_Teleporter_Out.SoundMix_Teleporter_Out")))

(event `self.Box_Enter.OnComponentBeginOverlap`
  (params (OverlappedComponent :type "PrimitiveComponent Object Reference") (OtherActor :type "Actor Object Reference") (OtherComp :type "PrimitiveComponent Object Reference") (OtherBodyIndex :type Integer) (bFromSweep :type Boolean) (SweepResult :type "HitResult Structure (by ref)"))
  (bind _asbp_character_berger (cast `/Game/_Project/Runtime/Code/BP/Characters/Berger/BP_Character_Berger` OtherActor)
    (:`then`
      (set `self.isBergerInside` true)
      (set `self.As BP Character Berger` _asbp_character_berger)
      (`/Engine/EditorBlueprintResources/StandardMacros.IsValid` (`self.PlayOnShep`)
        (:`Is Valid`)
        (:`Is Not Valid`
          (bind _returnvalue (`GameplayStatics.SpawnSoundAtLocation` (`self.WaveAsset`) (`self.K2_GetActorLocation`) (struct) 1.0 1.0 0.0 null null))
          (`GameplayStatics.SetSoundMixClassOverride` "/Game/_Project/Runtime/Assets/6_Audio/Mix/SoundMix/SFX/SoundMix_Teleporter_In.SoundMix_Teleporter_In" "/Game/_Project/Runtime/Assets/6_Audio/Mix/SoundClass/MIX_Class/MUS_IG.MUS_IG")
          (`GameplayStatics.SetSoundMixClassOverride` "/Game/_Project/Runtime/Assets/6_Audio/Mix/SoundMix/SFX/SoundMix_Teleporter_In.SoundMix_Teleporter_In" "/Game/_Project/Runtime/Assets/6_Audio/Mix/SoundClass/MIX_Class/AMB_Day_Mix.AMB_Day_Mix")
          (`GameplayStatics.SetSoundMixClassOverride` "/Game/_Project/Runtime/Assets/6_Audio/Mix/SoundMix/SFX/SoundMix_Teleporter_In.SoundMix_Teleporter_In" "/Game/_Project/Runtime/Assets/6_Audio/Mix/SoundClass/AMB_Night.AMB_Night")
          (`GameplayStatics.SetSoundMixClassOverride` "/Game/_Project/Runtime/Assets/6_Audio/Mix/SoundMix/SFX/SoundMix_Teleporter_In.SoundMix_Teleporter_In" "/Game/_Project/Runtime/Assets/6_Audio/Mix/SoundClass/MIX_Class/NPC_MIX.NPC_MIX")
          (`GameplayStatics.PushSoundMixModifier` "/Game/_Project/Runtime/Assets/6_Audio/Mix/SoundMix/SFX/SoundMix_Teleporter_In.SoundMix_Teleporter_In")
          (set `self.PlayOnShep` _returnvalue)
          (`KismetSystemLibrary.PrintString` "Audio_Hole_EnterBox" true true (struct :`R` 1.0 :`G` 1.0 :`B` 1.0 :`A` 1.0)))))
    (:`CastFailed`
      (`KismetSystemLibrary.PrintString` "Failed"))))

(event `CustomEvent`)

(event `self.Box_Exit_01.OnComponentBeginOverlap`
  (params (OverlappedComponent :type "PrimitiveComponent Object Reference") (OtherActor :type "Actor Object Reference") (OtherComp :type "PrimitiveComponent Object Reference") (OtherBodyIndex :type Integer) (bFromSweep :type Boolean) (SweepResult :type "HitResult Structure (by ref)"))
  ;[1 1 1] EXIT
  (cast `/Game/_Project/Runtime/Code/BP/Characters/Berger/BP_Character_Berger` OtherActor)
  (if (`self.isBergerInside`)
    (set `self.isBergerInside` false)
    (`AudioParameterControllerInterface.SetTriggerParameter` (`self.PlayOnShep`) "Stop")
    (`KismetSystemLibrary.PrintString` "Audio_Hole_ExitSphere" true true (struct :`R` 1.0 :`G` 1.0 :`B` 1.0 :`A` 1.0))
    (`GameplayStatics.SetSoundMixClassOverride` "/Game/_Project/Runtime/Assets/6_Audio/Mix/SoundMix/SFX/SoundMix_Teleporter_Out.SoundMix_Teleporter_Out" "/Game/_Project/Runtime/Assets/6_Audio/Mix/SoundClass/MIX_Class/MUS_IG.MUS_IG")
    (`GameplayStatics.SetSoundMixClassOverride` "/Game/_Project/Runtime/Assets/6_Audio/Mix/SoundMix/SFX/SoundMix_Teleporter_Out.SoundMix_Teleporter_Out" "/Game/_Project/Runtime/Assets/6_Audio/Mix/SoundClass/MIX_Class/AMB_Day_Mix.AMB_Day_Mix")
    (`GameplayStatics.SetSoundMixClassOverride` "/Game/_Project/Runtime/Assets/6_Audio/Mix/SoundMix/SFX/SoundMix_Teleporter_Out.SoundMix_Teleporter_Out" "/Game/_Project/Runtime/Assets/6_Audio/Mix/SoundClass/AMB_Night.AMB_Night")
    (`GameplayStatics.SetSoundMixClassOverride` "/Game/_Project/Runtime/Assets/6_Audio/Mix/SoundMix/SFX/SoundMix_Teleporter_Out.SoundMix_Teleporter_Out" "/Game/_Project/Runtime/Assets/6_Audio/Mix/SoundClass/MIX_Class/NPC_MIX.NPC_MIX")
    (`GameplayStatics.PushSoundMixModifier` "/Game/_Project/Runtime/Assets/6_Audio/Mix/SoundMix/SFX/SoundMix_Teleporter_Out.SoundMix_Teleporter_Out")))

(event `self.Box_Exit_02.OnComponentBeginOverlap`
  (params (OverlappedComponent :type "PrimitiveComponent Object Reference") (OtherActor :type "Actor Object Reference") (OtherComp :type "PrimitiveComponent Object Reference") (OtherBodyIndex :type Integer) (bFromSweep :type Boolean) (SweepResult :type "HitResult Structure (by ref)"))
  ;[1 1 1] EXIT
  (cast `/Game/_Project/Runtime/Code/BP/Characters/Berger/BP_Character_Berger` OtherActor)
  (if (`self.isBergerInside`)
    (set `self.isBergerInside` false)
    (`AudioParameterControllerInterface.SetTriggerParameter` (`self.PlayOnShep`) "Stop")
    (`GameplayStatics.SetSoundMixClassOverride` "/Game/_Project/Runtime/Assets/6_Audio/Mix/SoundMix/SFX/SoundMix_Teleporter_Out.SoundMix_Teleporter_Out" "/Game/_Project/Runtime/Assets/6_Audio/Mix/SoundClass/MIX_Class/MUS_IG.MUS_IG")
    (`GameplayStatics.SetSoundMixClassOverride` "/Game/_Project/Runtime/Assets/6_Audio/Mix/SoundMix/SFX/SoundMix_Teleporter_Out.SoundMix_Teleporter_Out" "/Game/_Project/Runtime/Assets/6_Audio/Mix/SoundClass/MIX_Class/AMB_Day_Mix.AMB_Day_Mix")
    (`GameplayStatics.SetSoundMixClassOverride` "/Game/_Project/Runtime/Assets/6_Audio/Mix/SoundMix/SFX/SoundMix_Teleporter_Out.SoundMix_Teleporter_Out" "/Game/_Project/Runtime/Assets/6_Audio/Mix/SoundClass/AMB_Night.AMB_Night")
    (`GameplayStatics.SetSoundMixClassOverride` "/Game/_Project/Runtime/Assets/6_Audio/Mix/SoundMix/SFX/SoundMix_Teleporter_Out.SoundMix_Teleporter_Out" "/Game/_Project/Runtime/Assets/6_Audio/Mix/SoundClass/MIX_Class/NPC_MIX.NPC_MIX")
    (`GameplayStatics.PushSoundMixModifier` "/Game/_Project/Runtime/Assets/6_Audio/Mix/SoundMix/SFX/SoundMix_Teleporter_Out.SoundMix_Teleporter_Out")
    (`KismetSystemLibrary.PrintString` "Audio_Hole_ExitSphere" true true (struct :`R` 1.0 :`G` 1.0 :`B` 1.0 :`A` 1.0))))

(fn `UserConstructionScript`)