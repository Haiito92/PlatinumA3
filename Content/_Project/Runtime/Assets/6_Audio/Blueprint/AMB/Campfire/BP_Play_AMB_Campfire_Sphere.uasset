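; Audio trigger actor that plays a looping 3D campfire ambience when the Berger (shepherd) or Chien (dog) character enters its sphere.
; Begin overlap flags the character and spawns the loop at the actor's location, unless the other character's sound already exists.
; End overlap sends a "Stop" trigger only when both flags are set and both sounds are valid.
; BeginPlay also spawns a sound at world origin, with no asset shown.
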(event `self.ReceiveBeginPlay`
  (`/Engine/EditorBlueprintResources/StandardMacros.IsValid` (`self.Play`)
    (:`Is Not Valid`
      (bind _returnvalue (`GameplayStatics.SpawnSoundAtLocation` null (0.0 0.0 0.0) (struct) 1.0 1.0 0.0 null null))
      (set `self.Play` _returnvalue))))

(event `self.Sphere1.OnComponentEndOverlap`
  (params (OverlappedComponent :type "PrimitiveComponent Object Reference") (OtherActor :type "Actor Object Reference") (OtherComp :type "PrimitiveComponent Object Reference") (OtherBodyIndex :type Integer))
  (if (and (`self.isDogInside`) (`self.isBergerInside`))
    (`/Engine/EditorBlueprintResources/StandardMacros.IsValid` (stale `self.Sphere1.OnComponentBeginOverlap` _returnvalue)
      (:`Is Valid`
        (`/Engine/EditorBlueprintResources/StandardMacros.IsValid` (stale `self.Sphere1.OnComponentBeginOverlap` _returnvalue_2)
          (:`Is Valid`
            (`AudioParameterControllerInterface.SetTriggerParameter` (stale `self.Sphere1.OnComponentBeginOverlap` _returnvalue) "Stop")
            (`AudioParameterControllerInterface.SetTriggerParameter` (stale `self.Sphere1.OnComponentBeginOverlap` _returnvalue_2) "Stop")
            (`KismetSystemLibrary.PrintString` "Audio_Hole_ExitSphere" true true (struct :`R` 1.0 :`G` 1.0 :`B` 1.0 :`A` 1.0))))))))

(event `self.Sphere1.OnComponentBeginOverlap`
  (params (OverlappedComponent :type "PrimitiveComponent Object Reference") (OtherActor :type "Actor Object Reference") (OtherComp :type "PrimitiveComponent Object Reference") (OtherBodyIndex :type Integer) (bFromSweep :type Boolean) (SweepResult :type "HitResult Structure (by ref)"))
  (bind _asbp_character_berger (cast `/Game/_Project/Runtime/Code/BP/Characters/Berger/BP_Character_Berger` OtherActor)
    (:`then`
      (set `self.isBergerInside` true)
      (set `self.As BP Character Berger` _asbp_character_berger)
      (`/Engine/EditorBlueprintResources/StandardMacros.IsValid` (`self.PlayOnDog`)
        (:`Is Not Valid`
          (bind _returnvalue (`GameplayStatics.SpawnSoundAtLocation` "/Game/_Project/Runtime/Assets/6_Audio/Event/AMB/Day/3D/Play_AMB_3D_Campfire_LP.Play_AMB_3D_Campfire_LP" (`self.K2_GetActorLocation`) (struct) 1.0 1.0 0.0 null null))
          (set `self.PlayOnShep` _returnvalue)
          (`KismetSystemLibrary.PrintString` "Audio_Hole_EnterSphere" true true (struct :`R` 1.0 :`G` 1.0 :`B` 1.0 :`A` 1.0)))))
    (:`CastFailed`
      (set `self.isBergerInside` false)
      (`/Engine/EditorBlueprintResources/StandardMacros.IsValid` (`self.PlayOnShep`)
        (:`Is Not Valid`
          (bind _asbp_character_chien (cast `/Game/_Project/Runtime/Code/BP/Characters/Chien/BP_Character_Chien` OtherActor)
            (:`then`
              (set `self.isDogInside` true)
              (set `self.As BP Character Chien` _asbp_character_chien)
              (bind _returnvalue_2 (`GameplayStatics.SpawnSoundAtLocation` "/Game/_Project/Runtime/Assets/6_Audio/Event/AMB/Day/3D/Play_AMB_3D_Campfire_LP.Play_AMB_3D_Campfire_LP" (`self.K2_GetActorLocation`) (struct) 1.0 1.0 0.0 null null))
              (set `self.PlayOnDog` _returnvalue_2))
            (:`CastFailed`
              (set `self.isDogInside` false))))))))

(fn `UserConstructionScript`)