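; Teleporter ambience actor that plays a positional sound when the Berger character enters its sphere.
; Begin overlap flags Berger as inside and spawns Play_AMB_Teleporter at the actor's location unless a Dog or Shep audio reference is already valid.
; End overlap sends a "Stop" audio trigger unless both inside flags are set, though only Berger's is ever set here.
; BeginPlay also makes a spawn-sound call at the world origin with no sound assigned.
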(event `self.ReceiveBeginPlay`
  (`/Engine/EditorBlueprintResources/StandardMacros.IsValid` (`self.Play`)
    (:`Is Not Valid`
      (bind _returnvalue (`GameplayStatics.SpawnSoundAtLocation` null (0.0 0.0 0.0) (struct) 1.0 1.0 0.0 null null))
      (set `self.Play` _returnvalue))))

(event `self.Sphere1.OnComponentEndOverlap`
  (params (OverlappedComponent :type "PrimitiveComponent Object Reference") (OtherActor :type "Actor Object Reference") (OtherComp :type "PrimitiveComponent Object Reference") (OtherBodyIndex :type Integer))
  (if (not (and (`self.isDogInside`) (`self.isBergerInside`)))
    (`/Engine/EditorBlueprintResources/StandardMacros.IsValid` (stale `self.Sphere1.OnComponentBeginOverlap` _returnvalue)
      (:`Is Valid`
        (`AudioParameterControllerInterface.SetTriggerParameter` (stale `self.Sphere1.OnComponentBeginOverlap` _returnvalue) "Stop"))
      (:`Is Not Valid`
        (`/Engine/EditorBlueprintResources/StandardMacros.IsValid` null
          (:`Is Valid`
            (`AudioParameterControllerInterface.SetTriggerParameter` (stale `self.Sphere1.OnComponentBeginOverlap` _returnvalue) "Stop")
            (`KismetSystemLibrary.PrintString` "Audio_Hole_ExitSphere" true true (struct :`R` 1.0 :`G` 1.0 :`B` 1.0 :`A` 1.0))))))))

(event `self.Sphere1.OnComponentBeginOverlap`
  (params (OverlappedComponent :type "PrimitiveComponent Object Reference") (OtherActor :type "Actor Object Reference") (OtherComp :type "PrimitiveComponent Object Reference") (OtherBodyIndex :type Integer) (bFromSweep :type Boolean) (SweepResult :type "HitResult Structure (by ref)"))
  (bind _asbp_character_berger (cast `/Game/_Project/Runtime/Code/BP/Characters/Berger/BP_Character_Berger` OtherActor))
  (set `self.isBergerInside` true)
  (set `self.As BP Character Berger` _asbp_character_berger)
  (`/Engine/EditorBlueprintResources/StandardMacros.IsValid` (`self.PlayOnDog`)
    (:`Is Not Valid`
      (`/Engine/EditorBlueprintResources/StandardMacros.IsValid` (`self.PlayOnShep`)
        (:`Is Not Valid`
          (bind _returnvalue (`GameplayStatics.SpawnSoundAtLocation` "/Game/_Project/Runtime/Assets/6_Audio/Event/AMB/Divers/Play_AMB_Teleporter.Play_AMB_Teleporter" (`self.K2_GetActorLocation`) (struct) 1.0 1.0 0.0 null null))
          (set `self.PlayOnShep` _returnvalue)
          (`KismetSystemLibrary.PrintString` "Audio_Hole_EnterSphere" true true (struct :`R` 1.0 :`G` 1.0 :`B` 1.0 :`A` 1.0)))))))

(fn `UserConstructionScript`)