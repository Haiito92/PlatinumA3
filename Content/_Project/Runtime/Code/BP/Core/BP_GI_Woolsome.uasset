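; BP_GI_Woolsome is the Woolsome Game Instance Blueprint that provides lookup of level info by index.
; GetLevelInfoByIndex searches the Levels map for a non-negative index and returns a found flag with the matching entry.
; GetCurrentLevelInfo passes CurrentLevelIndex into that lookup to return the current level's info.
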(fn `GetCurrentLevelInfo`
  (returns (FoundLevelInfo :type Boolean) (OutLevelInfo :type "/Game/_Project/Runtime/Code/Structs/GameLoop/S_FLevelInfo Structure"))
  (bind (_foundlevelinfo _outlevelinfo) (`self.GetLevelInfoByIndex` (`self.CurrentLevelIndex`)))
  (if _foundlevelinfo
    (return _foundlevelinfo _outlevelinfo)
    (else
      (return _foundlevelinfo))))

(fn `GetLevelInfoByIndex`
  (params (InLevelIndex :type Integer))
  (returns (FoundLevelInfo :type Boolean) (OutLevelInfo :type "/Game/_Project/Runtime/Code/Structs/GameLoop/S_FLevelInfo Structure"))
  (bind (_value _returnvalue) (`BlueprintMapLibrary.Map_Find` (`self.Levels`) (`local.InLevelIndex`)))
  (if (>= InLevelIndex 0)
    (if _returnvalue
      (return true _value)
      (else
        (return false)))))