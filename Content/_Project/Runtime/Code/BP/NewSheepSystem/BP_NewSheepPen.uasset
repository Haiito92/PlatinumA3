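; BP_NewSheepPen is a sheep pen actor that builds its fence along a spline.
; The construction script loops over PenFenceSpline, adding a spline mesh component with PenFenceMesh between each pair of consecutive points.
; Each segment is manually attached and takes world-space locations and tangents from the spline, with no segment added from last point to first.
; The event graph holds only disabled default events, so it has no runtime logic.
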(fn `UserConstructionScript`
  (for _index (range (+ (- (`SplineComponent.GetNumberOfSplinePoints` (`self.PenFenceSpline`)) 2) 1))
    (bind _returnvalue (`AddComponent|NODE_AddSplineMeshComponent-0` :`bManualAttachment` true))
    (`StaticMeshComponent.SetStaticMesh` _returnvalue (`|ConvertAsset` (`self.PenFenceMesh`)))
    (bind (_location _tangent) (`SplineComponent.GetLocationAndTangentAtSplinePoint` (`self.PenFenceSpline`) _index "World"))
    (bind (_location_2 _tangent_2) (`SplineComponent.GetLocationAndTangentAtSplinePoint` (`self.PenFenceSpline`) (+ _index 1) "World"))
    (`SplineMeshComponent.SetStartAndEnd` _returnvalue _location _tangent _location_2 _tangent_2 true)))